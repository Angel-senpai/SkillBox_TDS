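; Player controller that triggers test animation montages on the controlled top-down character.
; Space plays an ironsights or hip rifle fire montage depending on the character's AimEnabled flag.
; V plays a death montage on the same mesh.
; Both keys are bound directly in the event graph, and only montages play, with no firing or death logic.
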(event EventBeginPlay)

(event EventTick
  (params (DeltaSeconds :type Float%20%28single-precision%29)))

(event Input|KeyboardEvents|SpaceBar
  (params (Key :type Key%20Structure :default "None"))
  (:Pressed
    (bind _asbp_top_down_character (Utilities|Casting|CastToBP_TopDownCharacter (Pawn|GetControlledPawn)))
    (if (Variables|/Script/TDS.TDSCharacter|GetAimEnabled _asbp_top_down_character)
      (Animation|Montage|PlayMontage (Variables|/Script/Engine.Character|GetMesh _asbp_top_down_character) "/Game/Blueprints/Character/Mannequins/Animations/Montages/newFire_Rifle_Ironsights_Montage.newFire_Rifle_Ironsights_Montage")
      (else
        (Animation|Montage|PlayMontage (Variables|/Script/Engine.Character|GetMesh _asbp_top_down_character) "/Game/Blueprints/Character/Mannequins/Animations/Montages/newFire_Rifle_Hip_Montage.newFire_Rifle_Hip_Montage")))))

(event Input|KeyboardEvents|V
  (params (Key :type Key%20Structure :default "None"))
  (:Pressed
    (bind _asbp_top_down_character (Utilities|Casting|CastToBP_TopDownCharacter (Pawn|GetControlledPawn)))
    (Animation|Montage|PlayMontage (Variables|/Script/Engine.Character|GetMesh _asbp_top_down_character) "/Game/Blueprints/Character/Mannequins/Animations/Montages/newDeath_1_Montage.newDeath_1_Montage")))

(fn ConstructionScript)